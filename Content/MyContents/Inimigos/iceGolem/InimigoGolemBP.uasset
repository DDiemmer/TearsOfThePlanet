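; Ice golem enemy AI that patrols out and back from its spawn point and chases the player on sight.
; PawnSensing starts a recursive AIMoveTo chase and a looping distance-check timer.
; The timer picks by range, skipping while attacking: close plays a random guard or punch montage, mid-range prints placeholder growls.
; Beyond the far threshold, it drops the chase, clears the timer, returns to spawn and resumes patrolling.
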(event OnSeePawn(PawnSensing)
  (params (Pawn :type Pawn%20Object%20Reference))
  ;[1 1 1] Visao do inimigo
  (Utilities|Casting|CastToTakemisCharacterBP Pawn)
  (Variables|Default|SetinEniSight true)
  (Variables|Default|SetonSeekPlayer true)
  (CallFunction|SeekPlayer)
  (CallFunction|DistancePlayer))

(event Custom|SeekPlayer
  ;[1 1 1] Seek Player
  (if (Variables|Default|GetonSeekPlayer)
    (AI|AIMoveTo self "0, 0, 0" (Game|GetPlayerCharacter 0) 75.0 false
      (:then
        _)
      (:OnSuccess
        _)
      (:OnFail
        _))
    (Utilities|FlowControl|Delay 0.2)
    (CallFunction|SeekPlayer)
    (else
      (Development|PrintString "nao vejo nada" true true "(R=0.000000,G=0.660000,B=1.000000,A=1.000000)" 1.0)
      (Components|Movement|StopMovementImmediately (Variables|Character|GetCharacterMovement)))))

(event Custom|DistancePlayer
  ;[1 1 1] PLayer Distance Function
  (if (Variables|Default|GetonSeekPlayer)
    (Development|PrintString "onSeek")
    (if (Variables|Default|GettimerDistSetted)
      (Development|PrintString "ja foi iniciado ")
      (else
        (bind _returnvalue (Utilities|Time|SetTimerbyFunctionName 0 "PlayerDistance" 1.0 true))
        (Variables|Default|SetplayerDistHandle _returnvalue)
        (Variables|Default|SettimerDistSetted true)))
    (else
      (Development|PrintString "no seeking" true true "(R=0.000000,G=0.660000,B=1.000000,A=1.000000)" 1.0))))

(event Custom|ReturnToStartLocation
  ;[1 1 1] Return Position
  (if (not (Variables|Default|GetonSeekPlayer))
    (Utilities|FlowControl|Delay 1.5)
    (AI|AIMoveTo self (.Location (Math|Transform|BreakTransform (Variables|Default|GetstartTrasform))) 0 65.0 false
      (:OnSuccess
        (Utilities|FlowControl|Delay 3.0)
        (CallFunction|Patrol)))))

(event Custom|LongRange
  ;[1 1 1] Long Range action - Songs e etc
  (switch int (Math|Random|RandomIntegerinRange 0 2)
    (:0
      (Development|PrintString "rrruaaaahhh"))
    (:1
      (Development|PrintString "gggrrrrr"))
    (:2
      (Development|PrintString "crr crrk"))))

(event Custom|Patrol
  (bind _starttrasform (Variables|Default|GetstartTrasform))
  (bind (_location _rotation) (Math|Transform|BreakTransform _starttrasform))
  ;[1 1 1] Patrol
  (AI|AIMoveTo self (+ _location (* (Math|Vector|GetForwardVector _rotation) (Variables|Default|GetpatrolDistance))) 0 65.0 false
    (:OnSuccess
      _)
    (:OnFail
      _))
  (Utilities|FlowControl|Delay 1.3)
  (CallFunction|ReturntoStartLocation))

(event Custom|CloseRange
  ;[1 1 1] Close Range Attack or defenses
  (Variables|Default|SetisAttacking true)
  (switch int (Math|Random|RandomIntegerinRange 0 2)
    (:0
      (Variables|Default|SetattMontage "/Game/MyContents/Inimigos/iceGolem/AniMontage/BattlePosDef.BattlePosDef"))
    (:1
      (Variables|Default|SetattMontage "/Game/MyContents/Inimigos/iceGolem/AniMontage/PunchPos.PunchPos" :!label _label))
    (:2
      (goto _label)))
  (bind _returnvalue (Animation|PlayAnimMontage (Variables|Default|GetattMontage) 1.0 "None"))
  (Utilities|FlowControl|Delay _returnvalue)
  (Variables|Default|SetisAttacking false))

(event Custom|FarFarAway
  ;[1 1 1] Far far away range
  (Variables|Default|SetonSeekPlayer false)
  (Utilities|Time|ClearandInvalidateTimerbyHandle (Variables|Default|GetplayerDistHandle))
  (Variables|Default|SettimerDistSetted false)
  (Development|PrintString "retorna para a posicao  inicial ")
  (CallFunction|ReturntoStartLocation))

(event EventBeginPlay
  ;[1 1 1] Initialize
  (Variables|Default|SetisAlive true)
  (Variables|Default|SetinEniSight false)
  (Variables|Default|SetonSeekPlayer false)
  (Variables|Default|SettimerDistSetted false)
  (Variables|Default|SetstartTrasform (Transformation|GetWorldTransform (Variables|Collision|GetCapsuleComponent)))
  (Utilities|FlowControl|Delay 0.2)
  (CallFunction|DistancePlayer)
  (CallFunction|SeekPlayer)
  (Utilities|FlowControl|Delay 1.8)
  (if (not (Variables|Default|GetonSeekPlayer))
    (CallFunction|Patrol)))

(event Collision|EventActorBeginOverlap
  (params (OtherActor :type Actor%20Object%20Reference)))

(fn ConstructionScript)

(fn PlayerDistance
  (bind _returnvalue (Transformation|GetActorLocation))
  (bind _returnvalue_2 (Game|GetPlayerCharacter 0))
  (bind _returnvalue_3 (Transformation|GetActorLocation _returnvalue_2))
  (bind _returnvalue_4 (- _returnvalue _returnvalue_3))
  (bind _returnvalue_5 (Math|Vector|VectorLength _returnvalue_4))
  (if (Variables|Default|GetisAttacking)
    (Development|PrintString "atacando")
    (else
      ;[1 1 1] Detect Player Distance
      (bind _output_get (Variables|Default|Setdistance _returnvalue_5))
      ;[1 1 1] Attack Range Pick
      (if (> _returnvalue_5 4.5e+02)
        (if (> _returnvalue_5 2e+03)
          (CallFunction|FarFarAway)
          (Development|PrintString "far far away ")
          (else
            (CallFunction|LongRange)
            (Development|PrintString "long")))
        (else
          (CallFunction|CloseRange)
          (Development|PrintString "close ")))
      (Development|PrintString (Utilities|String|ToString(Float) _output_get) true true "(R=0.794276,G=0.664325,B=1.000000,A=1.000000)"))))