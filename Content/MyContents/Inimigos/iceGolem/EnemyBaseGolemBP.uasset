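; Ice golem enemy Blueprint that supplies close-range and long-range behaviors for the golem.
; CloseRange flags the golem as in action range, randomly plays a punch or defensive montage weighted toward the punch, and clears the flag after the montage's duration.
; LongRange only prints a random growl string, apparently a placeholder for sounds.
; Nothing in this graph triggers either event.
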(event Custom|LongRange
  ;[1 1 1] Long Range action - Songs e etc
  (switch int (Math|Random|RandomIntegerinRange 0 2)
    (:0
      (Development|PrintString "rrruaaaahhh"))
    (:1
      (Development|PrintString "gggrrrrr"))
    (:2
      (Development|PrintString "crr crrk"))))

(event Custom|CloseRange
  ;[1 1 1] Close Range Attack or defenses
  (Variables|Default|SetisInActionRange true)
  (switch int (Math|Random|RandomIntegerinRange 0 2)
    (:0
      (Variables|Default|SetAttMontage "/Game/MyContents/Inimigos/iceGolem/AniMontage/BattlePosDef.BattlePosDef"))
    (:1
      (Variables|Default|SetAttMontage "/Game/MyContents/Inimigos/iceGolem/AniMontage/PunchPos.PunchPos" :!label _label))
    (:2
      (goto _label)))
  (bind _returnvalue (Animation|PlayAnimMontage (Variables|Default|GetAttMontage) 1.0 "None"))
  (Utilities|FlowControl|Delay _returnvalue)
  (Variables|Default|SetisInActionRange false))

(event EventBeginPlay)

(event Collision|EventActorBeginOverlap
  (params (OtherActor :type Actor%20Object%20Reference)))

(event EventTick
  (params (DeltaSeconds :type Float%20%28single-precision%29)))

(fn ConstructionScript)