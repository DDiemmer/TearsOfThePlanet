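; BP_BaseInteractable is a base Blueprint for objects that the TakemisCharacterBP character can interact with.
; Overlap events on its InteratableArea component register and unregister the object with that character when it enters or leaves the area.
; SetHighLight toggles Render Custom Depth on InteractableMash to switch highlighting on or off.
; Particle visibility nodes are present but disconnected.
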(event OnComponentBeginOverlap(InteratableArea)
  (params (OverlappedComponent :type Primitive%20Component%20Object%20Reference) (OtherActor :type Actor%20Object%20Reference) (OtherComp :type Primitive%20Component%20Object%20Reference) (OtherBodyIndex :type Integer) (bFromSweep :type Boolean) (SweepResult :type Hit%20Result%20Structure%20%28by%20ref%29))
  (bind _astakemis_character_bp (Utilities|Casting|CastToTakemisCharacterBP OtherActor))
  (Class|BPIInteract|RegisterInteractable(Message) _astakemis_character_bp self))

(event OnComponentEndOverlap(InteratableArea)
  (params (OverlappedComponent :type Primitive%20Component%20Object%20Reference) (OtherActor :type Actor%20Object%20Reference) (OtherComp :type Primitive%20Component%20Object%20Reference) (OtherBodyIndex :type Integer))
  (bind _astakemis_character_bp (Utilities|Casting|CastToTakemisCharacterBP OtherActor))
  (Class|BPIInteract|UnregisterInteractable(Message) _astakemis_character_bp self))

(event EventBeginPlay)

(fn ConstructionScript)

(fn SetHighLight
  (params (HighLight :type Boolean))
  (Rendering|SetRenderCustomDepth (Variables|Default|GetInteractableMash) HighLight))